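; BP_SpawnManager is a spawn manager that keeps adding actors at random positions inside a fixed box-shaped volume; the spawned class is not shown.
; A one-second Delay on Tick throttles spawning into repeating waves of four SpawnActor calls.
; Each spawn takes a random location and a look-at rotation computed from a random point in that volume toward a fixed target just above the world origin.
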(event EventTick
  (params (DeltaSeconds :type Float%20%28single-precision%29))
  (bind _returnvalue (Math|Random|RandomFloatinRange -1e+03 1.1e+03))
  (bind _returnvalue_2 (Math|Random|RandomFloatinRange 1.5e+02 1.5e+03))
  (bind _returnvalue_3 (Math|Vector|MakeVector 0.0 0.0 9e+01))
  (bind _returnvalue_4 (Math|Random|RandomFloatinRange -2.6e+03 2.6e+03))
  (bind _returnvalue_5 (Math|Vector|MakeVector _returnvalue_4 _returnvalue _returnvalue_2))
  (bind _returnvalue_6 (Math|Rotator|FindLookatRotation _returnvalue_5 _returnvalue_3))
  (Utilities|FlowControl|Delay 1.0)
  (Game|SpawnActorfromClass "/Game/FPS/Blueprints/Game/Targets/BP_Basics.BP_Basics_C" (Math|Transform|MakeTransform _returnvalue_5 _returnvalue_6 "1.000000,1.000000,1.000000") "Undefined" "MultiplyWithRoot" 0 0)
  (Game|SpawnActorfromClass "/Game/FPS/Blueprints/Game/Targets/BP_Apples.BP_Apples_C" (Math|Transform|MakeTransform _returnvalue_5 _returnvalue_6 "1.000000,1.000000,1.000000") "Undefined" "MultiplyWithRoot" 0 0)
  (Game|SpawnActorfromClass "/Game/FPS/Blueprints/Game/Targets/BP_Bombs.BP_Bombs_C" (Math|Transform|MakeTransform _returnvalue_5 _returnvalue_6 "1.000000,1.000000,1.000000") "Undefined" "MultiplyWithRoot" 0 0)
  (Game|SpawnActorfromClass "/Game/FPS/Blueprints/Game/Targets/BP_Bottles.BP_Bottles_C" (Math|Transform|MakeTransform _returnvalue_5 _returnvalue_6 "1.000000,1.000000,1.000000") "Undefined" "MultiplyWithRoot" 0 0))

(fn ConstructionScript)
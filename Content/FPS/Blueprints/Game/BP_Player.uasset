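; BP_Player is the first-person shooter player Blueprint, handling look input and a starting weapon.
; On BeginPlay it spawns the StartingGun class, stores it as GunRef and snaps it to GunSpawnPoint.
; Horizontal and vertical look axes drive controller yaw and pitch.
; Firing is a placeholder: while the Fire axis is held, a short Delay throttles a repeated "Fire" debug print, without calling the gun.
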(event EventBeginPlay
  (Development|PrintString "Spawing BP_Player")
  (CallFunction|SpawningStartingGun (Variables|Config|GetStarting%20Gun)))

(event Input|AxisEvents|InputAxisLookHorizontal
  (params (AxisValue :type Float%20%28single-precision%29))
  ;[0.15 0.15 0.15 0.5] Looking
  (Pawn|Input|AddControllerYawInput AxisValue))

(event Input|AxisEvents|InputAxisFire
  (params (AxisValue :type Float%20%28single-precision%29))
  ;[0.15 0.15 0.15 0.5] Shooting
  (if (> AxisValue 0.0)
    (Utilities|FlowControl|Delay 0.2)
    (Development|PrintString "Fire")))

(event Input|AxisEvents|InputAxisLookVertical
  (params (AxisValue :type Float%20%28single-precision%29))
  ;[0.15 0.15 0.15 0.5] Looking
  (Pawn|Input|AddControllerPitchInput AxisValue))

(fn ConstructionScript)

(fn SpawningStartingGun
  (params (StartingGun :type Actor%20Class%20Reference))
  (bind _returnvalue (Game|SpawnActorfromClass StartingGun (Math|Transform|MakeTransform "0, 0, 0") "Undefined" "MultiplyWithRoot" 0 0))
  (bind _output_get (Variables|Default|SetGunRef _returnvalue))
  (Transformation|AttachComponentToComponent _output_get (Variables|Default|GetGunSpawnPoint) "None" "SnapToTarget" "SnapToTarget" "SnapToTarget" true))
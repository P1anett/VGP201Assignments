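; Game mode for a timed score-attack round in an FPS project, opening the game-over map when the timer hits zero.
; BeginPlay loads or creates the save, spawns BP_SpawnManager and the HUD widget, then resets the saved current score.
; Tick drives the countdown through a one-second Delay and refreshes the score display.
; AddScore clamps and saves the score, also saving any new high score.
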(event EventTick
  (params (DeltaSeconds :type Float%20%28single-precision%29))
  (CallFunction|GameOver)
  (CallFunction|UpdateScore)
  (Utilities|DecreaseTimer))

(event EventBeginPlay
  (bind _returnvalue (SaveGame|DoesSaveGameExist (Variables|Default|GetSaveSlotName)))
  (if _returnvalue
    (bind _returnvalue_2 (SaveGame|LoadGamefromSlot (Variables|Default|GetSaveSlotName)))
    (bind _asbp_save_data (Utilities|Casting|CastToBP_SaveData _returnvalue_2))
    (Variables|Config|SetHighScore (Variables|/Game/FPS/Blueprints/Game/BP_SaveData.BP_SaveData_C|GetSHighScore _asbp_save_data))
    (else
      (bind _returnvalue_3 (SaveGame|CreateSaveGameObject "/Game/FPS/Blueprints/Game/BP_SaveData.BP_SaveData_C"))
      (Variables|Config|SetHighScore 0)
      (SaveGame|SaveGametoSlot _returnvalue_3 (Variables|Default|GetSaveSlotName))))
  (Development|PrintString "Spawning BP_Gamemode" true true "(R=0.000000,G=0.660000,B=1.000000,A=1.000000)" 5.0)
  (Game|SpawnActorfromClass "/Game/FPS/Blueprints/Game/BP_SpawnManager.BP_SpawnManager_C" (Math|Conversions|ToTransform(Vector) (Transformation|GetWorldLocation (Variables|Default|GetDefaultSceneRoot))) "Undefined" "MultiplyWithRoot" 0 0)
  (CallFunction|SpawnGUI)
  (CallFunction|UpdateTimer)
  (CallFunction|UpdateScore)
  (CallFunction|UpdateHighScore)
  (bind _returnvalue_4 (SaveGame|LoadGamefromSlot (Variables|Default|GetSaveSlotName)))
  (bind _asbp_save_data_2 (Utilities|Casting|CastToBP_SaveData _returnvalue_4))
  (Variables|/Game/FPS/Blueprints/Game/BP_SaveData.BP_SaveData_C|SetCurrentScore _asbp_save_data_2 0)
  (SaveGame|SaveGametoSlot _asbp_save_data_2 (Variables|Default|GetSaveSlotName)))

(fn ConstructionScript)

(fn UpdateTimer
  (bind _aswbp_game_menu (Utilities|Casting|CastToWBP_GameMenu (Variables|Default|GetMenu%20Ref)))
  (Default|UpdateTimer _aswbp_game_menu (Variables|config|GetGameTimer)))

(fn SpawnGUI
  (bind _returnvalue (Game|GetPlayerController 0))
  (bind _returnvalue_2 (UserInterface|CreateWidget "/Game/FPS/Blueprints/Game/GUI/WBP_GameMenu.WBP_GameMenu_C"))
  (bind _output_get (Variables|Default|SetMenu%20Ref _returnvalue_2))
  (UserInterface|Viewport|AddtoViewport _output_get 0)
  (Input|SetInputModeGameOnly _returnvalue false)
  (Variables|/Script/Engine.PlayerController|SetbShowMouseCursor _returnvalue false))

(fn UpdateScore
  (bind _aswbp_game_menu (Utilities|Casting|CastToWBP_GameMenu (Variables|Default|GetMenu%20Ref)))
  (Default|UpdateScore _aswbp_game_menu (Variables|config|GetScore)))

(fn GameOver
  (if (== (Variables|config|GetGameTimer) 0)
    (Game|OpenLevel(byObjectReference) "/Game/FPS/Maps/GameOverMap.GameOverMap")))

(fn AddScore
  (params (ScoreValue :type Integer))
  (Variables|config|SetScore (Math|Integer|Clamp(Integer) (+ (Variables|config|GetScore) ScoreValue) 0 2147483647))
  (CallFunction|UpdateScore)
  (bind _returnvalue (SaveGame|LoadGamefromSlot (Variables|Default|GetSaveSlotName)))
  (bind _asbp_save_data (Utilities|Casting|CastToBP_SaveData _returnvalue))
  (Variables|/Game/FPS/Blueprints/Game/BP_SaveData.BP_SaveData_C|SetCurrentScore _asbp_save_data (Variables|config|GetScore))
  (SaveGame|SaveGametoSlot _asbp_save_data (Variables|Default|GetSaveSlotName))
  (if (> (Variables|config|GetScore) (Variables|Config|GetHighScore))
    (Variables|Config|SetHighScore (Variables|config|GetScore))
    (CallFunction|SaveHighScore)
    (CallFunction|UpdateHighScore)))

(fn UpdateHighScore
  (bind _aswbp_game_menu (Utilities|Casting|CastToWBP_GameMenu (Variables|Default|GetMenu%20Ref)))
  (Default|UpdateHighScore _aswbp_game_menu (Variables|Config|GetHighScore)))

(fn SaveHighScore
  (bind _returnvalue (SaveGame|DoesSaveGameExist (Variables|Default|GetSaveSlotName)))
  (if _returnvalue
    (bind _returnvalue_2 (SaveGame|LoadGamefromSlot (Variables|Default|GetSaveSlotName)))
    (bind _asbp_save_data (Utilities|Casting|CastToBP_SaveData _returnvalue_2))
    (bind _output_get (Variables|/Game/FPS/Blueprints/Game/BP_SaveData.BP_SaveData_C|SetSHighScore _asbp_save_data (Variables|Config|GetHighScore)))
    (Development|PrintString (Utilities|String|ToString(Integer) _output_get))
    (SaveGame|SaveGametoSlot _asbp_save_data (Variables|Default|GetSaveSlotName))))